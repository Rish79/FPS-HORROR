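; FeedLocationBP is an interactable feeding spot that restores the horror game's player character.
; Box overlap with an FPSHorrorCharacter caches that character and enables input on this actor for the first player controller.
; Pressing E then sets the cached character's Health to a fixed value and increases CurrentPeers, with no cooldown or use limit.
; Actor end overlap by that character type calls DisableInput without specifying a controller.
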(event `self.ReceiveBeginPlay`)

(event `self.ReceiveActorBeginOverlap`
  (params (OtherActor :type "Actor Object Reference")))

(event `self.Box.OnComponentBeginOverlap`
  (params (OtherActor :type "Actor Object Reference") (OtherComp :type "PrimitiveComponent Object Reference") (OtherBodyIndex :type Integer) (bFromSweep :type Boolean) (SweepResult :type "HitResult Structure (by ref)"))
  (bind _asfpshorror_character (cast `FPSHorrorCharacter` OtherActor))
  (`self.EnableInput` (`GameplayStatics.GetPlayerController` 0)))

(event `Key|E`
  (params (Key :type "Key Structure" :default "AnyKey"))
  (:`Pressed`
    (set `FPSHorrorCharacter.Health` 100.0 (stale `self.Box.OnComponentBeginOverlap` _asfpshorror_character))
    (set `FPSHorrorCharacter.CurrentPeers` (+ (`FPSHorrorCharacter.CurrentPeers` (stale `self.Box.OnComponentBeginOverlap` _asfpshorror_character)) 10.0) (stale `self.Box.OnComponentBeginOverlap` _asfpshorror_character))))

(event `self.ReceiveActorEndOverlap`
  (params (OtherActor :type "Actor Object Reference"))
  (cast `FPSHorrorCharacter` OtherActor)
  (`self.DisableInput` null))

(fn `UserConstructionScript`)